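; BP_Car_Child1 is a car Blueprint child that acts as a flying vehicle, lifting its pickup mesh into the air when play begins.
; BeginPlay prints "Plane flies", stores the mesh's world location and plays a Timeline.
; Each Timeline update lerps the mesh from that start toward a fixed world height, keeping X and Y unchanged and moving without sweep.
; The construction script only calls the parent's.
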(event EventBeginPlay
  (Development|PrintString "Plane flies")
  (bind _output_get (Variables|Default|SetStartPosition (Transformation|GetWorldLocation (Variables|Default|GetSK_veh_PickupOld_01))))
  (bind _newtrack_0 (Timeline|Timeline Play)
    (:Update
      (Transformation|SetWorldLocation (Variables|Default|GetSK_veh_PickupOld_01) (Math|Vector|Lerp(Vector) _output_get (Math|Vector|MakeVector (.x (Variables|Default|GetStartPosition)) (.y (Variables|Default|GetStartPosition)) 5e+02) _newtrack_0) false false))))

(fn ConstructionScript
  (|CallParentFunction))
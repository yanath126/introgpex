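; BP_Grenade is a physics grenade that knocks physics objects around with a delayed radial blast.
; On BeginPlay it moves just in front of the player's first-person camera and launches its Sphere with an impulse along fixed world X.
; After a short delay it gathers physics-body components in a very large sphere overlap and applies a linear-falloff radial impulse to each.
; It applies no damage and never destroys itself.
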(event EventBeginPlay
  (bind _sphere (Variables|Default|GetSphere))
  (bind _player (Variables|Default|Getplayer))
  (bind _returnvalue (Transformation|GetWorldLocation _sphere))
  (bind _firstpersoncamera (Variables|/Game/FirstPerson/Blueprints/BP_FirstPersonCharacter.BP_FirstPersonCharacter_C|GetFirstPersonCamera _player))
  (Transformation|SetActorLocation (+ (* (Math|Vector|GetForwardVector _firstpersoncamera) 5e+01) (Transformation|GetWorldLocation _firstpersoncamera)) false false)
  (Physics|AddImpulse (Variables|Default|GetSphere) "50000.000000,0.000000,0.000000" "None" false)
  (Utilities|FlowControl|Delay 2.0)
  (bind _outcomponents (Collision|SphereOverlapComponents _returnvalue 5e+05 (Utilities|Array|MakeArray "ObjectTypeQuery4")))
  (for _array_element _outcomponents
    (Physics|AddRadialImpulse _array_element _returnvalue 3.5e+03 1e+05 "RIF_Linear" false)))

(fn ConstructionScript)
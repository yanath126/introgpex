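; BP_PUCoin is a coin pickup that hides its sphere and adds to a score when a BP_FirstPersonCharacter overlaps it.
; The overlap sets CoinPickedUp, enables input for player 0, increments the coin's own Score variable and prints it to screen.
; A Respawn event shows the sphere again after a delay; only visibility toggles, with collision untouched and CoinPickedUp never reset.
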(event Custom|Respawn
  (Utilities|FlowControl|Delay 5.0)
  (Rendering|SetVisibility (Variables|Default|GetSphere) true false))

(event Collision|EventActorBeginOverlap
  (params (OtherActor :type Actor%20Object%20Reference))
  (Utilities|Casting|CastToBP_FirstPersonCharacter OtherActor)
  (Variables|Default|SetCoin%20picked%20up true)
  (Rendering|SetVisibility (Variables|Default|GetSphere) false false)
  (CallFunction|Respawn)
  (Input|EnableInput (Game|GetPlayerController 0))
  (if (Variables|Default|GetCoin%20picked%20up)
    (bind _result (Math|Integer|IncrementInt (Variables|Default|GetScore))
      (:%20%20
        (Development|PrintString (Utilities|String|ToString(Integer) _result))))
    (else
      (Development|PrintString (Utilities|String|ToString(Integer) (Variables|Default|GetScore))))))

(fn ConstructionScript)
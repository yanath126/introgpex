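; BP_movingledge is a ledge actor whose Cube slides along the world Y axis once play begins.
; BeginPlay caches the Cube's start location, then the Move timeline lerps it toward a fixed world Y coordinate, keeping X and Z unchanged, without sweeping.
; A spawn event creates another BP_movingledge at the Cube's current location; nothing in this Blueprint calls it.
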(event Custom|spawn
  (Game|SpawnActorfromClass "BP_movingledge_C" (Math|Conversions|ToTransform(Vector) (Transformation|GetWorldLocation (Variables|Default|GetCube))) "Undefined" "MultiplyWithRoot" 0 0))

(event EventBeginPlay
  (Variables|Default|Setstarposition (Transformation|GetWorldLocation (Variables|Default|GetCube)))
  (bind _newtrack_1 (Timeline|move Play)
    (:Update
      (Transformation|SetWorldLocation (Variables|Default|GetCube) (Math|Vector|Lerp(Vector) (Variables|Default|Getstarposition) (Math|Vector|MakeVector (.x (Variables|Default|Getstarposition)) 2e+02 (.z (Variables|Default|Getstarposition))) _newtrack_1) false false))))

(fn ConstructionScript)
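; BP_trigger1 is a trigger actor that controls the picked-up state and visibility of a referenced Paper actor.
; When the first-person character begins overlapping, it hides the paper, sets PaperPickedup and enables its own input.
; While input is enabled, F drives a FlipFlop that alternately shows and hides the paper, updating the flag to match.
; Ending the overlap disables input again, limiting the toggle to the trigger area.
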(event Collision|EventActorEndOverlap
  (params (OtherActor :type Actor%20Object%20Reference))
  (Utilities|Casting|CastToBP_FirstPersonCharacter OtherActor)
  (Input|DisableInput (Game|GetPlayerController 0)))

(event Collision|EventActorBeginOverlap
  (params (OtherActor :type Actor%20Object%20Reference))
  (Utilities|Casting|CastToBP_FirstPersonCharacter OtherActor)
  (Variables|Default|SetPaper%20pickedup true)
  (Rendering|SetActorHiddenInGame (Variables|Default|Getpaper) true)
  (Input|EnableInput (Game|GetPlayerController 0)))

(event Input|KeyboardEvents|F
  (params (Key :type Key%20Structure :default "None"))
  (bind _paper (Variables|Default|Getpaper))
  (:Pressed
    (Utilities|FlowControl|FlipFlop
      (:A
        (Rendering|SetActorHiddenInGame _paper false)
        (Variables|Default|SetPaper%20pickedup false))
      (:B
        (Rendering|SetActorHiddenInGame _paper true)
        (Variables|Default|SetPaper%20pickedup true)))))

(fn ConstructionScript)